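; Actor component for VR hands that simulates a realistic grab by snapping the hand mesh to grab components and wrapping fingers around objects.
; SimGrabOnTick finds the grab component near the motion controller and snaps, simulates fingers or stops, based on its snap type.
; While simulating, per-bone box traces curl or back off each three-joint finger, feeding alphas to the hand AnimBP.
; When stopped, fingers ease back open.
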(event `self.ReceiveTick`
  (params (DeltaSeconds :type "Float (single-precision)"))
  ;[0 1 0.5702] Grab simulation control
  (`|ExecutionSequence`
    (:`then_0`
      (`self.HandMeshToControlRef`
        (:`then`
          (if (`self.SimulateGrab`)
            (`/Engine/EditorBlueprintResources/StandardMacros.Gate` false :!label _label
              (:`Exit`
                (`self.HCControl Fingers`)
                (`self.HCUpdate Hand Anim BP`)
                (`|ExecutionSequence`
                  (:`then_0`
                    (bind _grab_component_ref (`self.Grab Component Ref`)
                      (:`then`
                        (bind _stopfingersimafterdelay (`/Game/VRHandGrab/Blueprints/ACGrabComponent.StopFingerSimAfterDelay` _grab_component_ref))
                        ;[1 1 1] Stom simulating after delay if Grab type = "snap"
                        (if (> _stopfingersimafterdelay 0.0)
                          (`KismetSystemLibrary.Delay` _stopfingersimafterdelay)
                          (if (`self.HandSnappedToObject`)
                            (goto _label :!via `Close`))))
                      (:`else`)))
                  (:`then_1`
                    (goto _label_2 :!via `Open`)))))
            (else
              (`|ExecutionSequence`
                (:`then_0`
                  ;[1 1 1] Restore hand pose smoothly
                  (if (not (`self.SimulateGrab`))
                    (`/Engine/EditorBlueprintResources/StandardMacros.Gate` true :!label _label_2
                      (:`Exit`
                        (if (`self.CheckFingersAlpha`)
                          (for (_ _array_index) (`self.S_HandAllBoneNamesBase`)
                            (`self.HCUndoMoveFinger` _array_index 0.05) ; Undo
                            (`self.HCUpdate Hand Anim BP`))
                          (else
                            (goto _label_2 :!via `Close`)))))))
                (:`then_1`
                  (goto _label :!via `Open`))))))
        (:`else`)))))

(event `StartSimGrab`
  (params (HandMeshToControlRef :type "SkeletalMeshComponent Object Reference"))
  ;[0 1 0.5702] Grab Simulation events (called by user in vr)
  (set `self.HandMeshToControlRef` HandMeshToControlRef)
  (set `self.SimulateGrab` true)
  (`|ExecutionSequence`
    (:`then_0`
      (`/Engine/EditorBlueprintResources/StandardMacros.DoOnce` false :!label _label_3
        (:`Completed`
          (`self.OnSimGrabStarted`))))
    (:`then_1`
      (goto _label_4 :!via `Reset`))))

(event `StopSimGrab`
  ;[0 1 0.5702] Grab Simulation events (called by user in vr)
  (set `self.CurrCustomFingerAlphaInterp` 0.0)
  (set `self.SimulateGrab` false)
  (`|ExecutionSequence`
    (:`then_0`
      (`/Engine/EditorBlueprintResources/StandardMacros.DoOnce` false :!label _label_4
        (:`Completed`
          (`self.OnSimGrabStopped`))))
    (:`then_1`
      (goto _label_3 :!via `Reset`))))

(event `SnapHandToGrabComp`
  (params (GtabComponentRef :type "SceneComponent Object Reference"))
  (bind _snapped (`self.HCSnapHandMeshToObj` GtabComponentRef (`self.HandMeshToControlRef`) (`self.Hand Rel Transform Default`)))
  (bind _output_get (set `self.HandSnappedToObject` _snapped))
  (if _output_get
    (`self.StartSimGrab` (`self.HandMeshToControlRef`))
    (else
      (`self.StopSimGrab`))))

(event `TryResetHandRelTransform`
  (`/Engine/EditorBlueprintResources/StandardMacros.IsValid` (`self.Nearest Component`)
    (:`Is Valid`
      (goto _label_5 :!via `Reset`))
    (:`Is Not Valid`
      ;[1 1 1] Reset if there are no grab components near the hand
      (`/Engine/EditorBlueprintResources/StandardMacros.DoOnce` false :!label _label_5
        (:`Completed`
          (`SceneComponent.K2_SetRelativeTransform` (`self.HandMeshToControlRef`) (`self.Hand Rel Transform Default`) false false))))))

(fn `CheckFingersAlpha`
  (returns (Continue :type Boolean))
  (locals (RestoreNotFinished :type Boolean :default false))
  (for _array_element (`self.S_HandAllBoneNamesBase`)
    (if (!= (`.Alpha_38_5439CFAD46D58980D75259BC215F4D5C` (break `/Game/VRHandGrab/Blueprints/Structures/S_HandBoneRotation` _array_element)) 0.0)
      (set `local.RestoreNotFinished` true)
      (break)))
  (return (`local.RestoreNotFinished`)))

(fn `FingersMovementNew`
  (params (FingerIndex :type Integer :default 0))
  (locals (Index01 :type Integer) (Index02 :type Integer) (Index03 :type Integer))
  (bind (_output_bonename _output_alpha _output_blocked) (break `/Game/VRHandGrab/Blueprints/Structures/S_HandBoneRotation` (`|GetArrayItem` (`self.S_HandAllBoneNamesBase`) (`local.Index03`))))
  (bind (_output_bonename_2 _output_alpha_2 _output_blocked_2 _output_distance) (break `/Game/VRHandGrab/Blueprints/Structures/S_HandBoneRotation` (`|GetArrayItem` (`self.S_HandAllBoneNamesBase`) (`local.Index01`))))
  (bind (_output_bonename_3 _output_alpha_3 _output_blocked_3 _output_distance_2) (break `/Game/VRHandGrab/Blueprints/Structures/S_HandBoneRotation` (`|GetArrayItem` (`self.S_HandAllBoneNamesBase`) (`local.Index03`))))
  (bind (_output_bonename_4 _output_alpha_4 _output_blocked_4) (break `/Game/VRHandGrab/Blueprints/Structures/S_HandBoneRotation` (`|GetArrayItem` (`self.S_HandAllBoneNamesBase`) (`local.Index02`))))
  (bind (_output_bonename_5 _output_alpha_5 _output_blocked_5) (break `/Game/VRHandGrab/Blueprints/Structures/S_HandBoneRotation` (`|GetArrayItem` (`self.S_HandAllBoneNamesBase`) (`local.Index03`))))
  (bind (_output_bonename_6 _output_alpha_6 _output_blocked_6) (break `/Game/VRHandGrab/Blueprints/Structures/S_HandBoneRotation` (`|GetArrayItem` (`self.S_HandAllBoneNamesBase`) (`local.Index03`))))
  (bind (_output_bonename_7 _output_alpha_7 _output_blocked_7 _output_distance_3) (break `/Game/VRHandGrab/Blueprints/Structures/S_HandBoneRotation` (`|GetArrayItem` (`self.S_HandAllBoneNamesBase`) (`local.Index02`))))
  (bind _output_get (set `local.Index01` FingerIndex))
  (bind _output_get_2 (set `local.Index02` (+ _output_get 1)))
  (set `local.Index03` (+ _output_get_2 1))
  ;[1 0.1281 0] Undo
  (`|ExecutionSequence`
    (:`then_0`
      (if (and (== _output_distance 0.0) _output_blocked_2)
        (`self.HCUndoMoveFinger` (`local.Index01`) 0.01) ; Undo
        (else
          ;[1 0.1281 0] Move fingers
          (if (and (not _output_blocked_4) (not _output_blocked_5))
            (`self.HCMoveFinger` (`local.Index01`) (`self.FingerMoveSpeed`)) ; move until touches surface
          ))))
    (:`then_1`
      (if (and (== _output_distance_3 0.0) _output_blocked_7)
        (`self.HCUndoMoveFinger` (`local.Index02`) 0.01) ; Undo
        (`self.HCUndoMoveFinger` (`local.Index01`) 0.01) ; Undo
        (elif (not _output_blocked_6)
          (`self.HCMoveFinger` (`local.Index02`) (`self.FingerMoveSpeed`)) ; move until touches surface
        )))
    (:`then_2`
      (if (and (== _output_distance_2 0.0) _output_blocked_3)
        (`self.HCUndoMoveFinger` (`local.Index03`) 0.01) ; Undo
        (`self.HCUndoMoveFinger` (`local.Index02`) 0.01) ; Undo
        (`self.HCUndoMoveFinger` (`local.Index01`) 0.01) ; Undo
        (elif (not _output_blocked)
          (`self.HCMoveFinger` (`local.Index03`) (`self.FingerMoveSpeed`)) ; move until touches surface
        )))))

(fn `HCControl Fingers`
  (locals (DistanceToSurface :type "Float (double-precision)" :default 0.0))
  (bind _s_handallbonenamesbase (`self.S_HandAllBoneNamesBase`))
  ;[1 0.1281 0] Init hand bones name
  (if (not (`self.HandBoneNamesInitialized`))
    (bind _handmeshtocontrolref (`self.HandMeshToControlRef`)
      (:`then`
        (bind _handbones (message `/Game/VRHandGrab/Blueprints/BPI_HandAnim.GetHandBonesName` (`SkeletalMeshComponent.GetAnimInstance` _handmeshtocontrolref)))
        (set `self.S_HandAllBoneNamesBase` _handbones)
        (set `self.HandBoneNamesInitialized` true))
      (:`else`
        (set `self.HandBoneNamesInitialized` false)))
    (else
      ;[1 0.1281 0] Fingers control
      (`|ExecutionSequence`
        (:`then_0`
          ;[1 0.1281 0] Trace
          (for (_array_element _array_index) _s_handallbonenamesbase
            (bind (_traceblocked _distancebtwstarttoimpact) (`self.HCTraceIfTouchedSurfaceByIndex` (`self.Trace Distance`) (`self.Move Start Trace Frwd`) _array_index))
            (bind _structout (setmembers `/Game/VRHandGrab/Blueprints/Structures/S_HandBoneRotation` :`StructRef` _array_element :`Blocked` _traceblocked :`Distance` _distancebtwstarttoimpact))
            (`KismetArrayLibrary.Array_Set` _s_handallbonenamesbase _array_index _structout)))
        (:`then_1`
          (`self.FingersMovementNew` (`self.CurIndForIndex`)))
        (:`then_2`
          (`self.FingersMovementNew` (`self.CurIndForMiddle`)))
        (:`then_3`
          (`self.FingersMovementNew` (`self.CurIndForRing`)))
        (:`then_4`
          (`self.FingersMovementNew` (`self.CurIndForPinky`)))
        (:`then_5`
          (`self.FingersMovementNew` (`self.CurIndForThumb`)))))))

(fn `HCMoveFinger`
  (params (Index :type Integer) (FingerMovementSpeed :type "Float (double-precision)" :default 0.1))
  (returns (Success :type Boolean) (IndexModified :type Integer) (Alpha :type "Float (double-precision)"))
  (locals (ValidIndex :type Integer :default 0))
  (bind _s_handallbonenamesbase (`self.S_HandAllBoneNamesBase`))
  (bind _output (`|GetArrayItem` _s_handallbonenamesbase (`local.ValidIndex`)))
  (bind _returnvalue (`KismetMathLibrary.FClamp` (+ (`.Alpha_38_5439CFAD46D58980D75259BC215F4D5C` (break `/Game/VRHandGrab/Blueprints/Structures/S_HandBoneRotation` _output)) (* FingerMovementSpeed (`GameplayStatics.GetWorldDeltaSeconds`) 100.0))))
  (set `local.ValidIndex` Index)
  (if (`KismetArrayLibrary.Array_IsValidIndex` _s_handallbonenamesbase (`local.ValidIndex`))
    (bind _structout (setmembers `/Game/VRHandGrab/Blueprints/Structures/S_HandBoneRotation` :`StructRef` _output :`Alpha` _returnvalue))
    (`KismetArrayLibrary.Array_Set` _s_handallbonenamesbase (`local.ValidIndex`) _structout)
    (return true (`local.ValidIndex`) _returnvalue)
    (else
      (return false 0 0.0))))

(fn `HCRestoreFingersMovement`
  (bind _s_handallbonenamesbase (`self.S_HandAllBoneNamesBase`))
  (for (_array_element _array_index) _s_handallbonenamesbase
    (bind _structout (setmembers `/Game/VRHandGrab/Blueprints/Structures/S_HandBoneRotation` :`StructRef` _array_element :`Alpha` 0.0))
    (`KismetArrayLibrary.Array_Set` _s_handallbonenamesbase _array_index _structout))
  (`self.HCUpdate Hand Anim BP`)
  (return))

(fn `HCSetFingerAlpha`
  (params (Index :type Integer) (FingerAlpha :type "Float (double-precision)" :default 0.1))
  (returns (Success :type Boolean) (IndexModified :type Integer))
  (locals (ValidIndex :type Integer :default 0))
  (bind _s_handallbonenamesbase (`self.S_HandAllBoneNamesBase`))
  (set `local.ValidIndex` Index)
  (if (`KismetArrayLibrary.Array_IsValidIndex` _s_handallbonenamesbase (`local.ValidIndex`))
    (bind _structout (setmembers `/Game/VRHandGrab/Blueprints/Structures/S_HandBoneRotation` :`StructRef` (`|GetArrayItem` _s_handallbonenamesbase (`local.ValidIndex`)) :`Alpha` FingerAlpha))
    (`KismetArrayLibrary.Array_Set` _s_handallbonenamesbase (`local.ValidIndex`) _structout)
    (return true (`local.ValidIndex`))
    (else
      (return false 0))))

(fn `HCSnapHandMeshToObj`
  (params (GtabComponentRef :type "SceneComponent Object Reference") (HandMeshLocal :type "SkeletalMeshComponent Object Reference") (HandDefaultRelTransf :type "Transform Structure"))
  (returns (Snapped :type Boolean))
  (locals (HandMeshRefLocal :type "SkeletalMeshComponent Object Reference") (GrabCompRefLocal :type "SceneComponent Object Reference"))
  (bind _returnvalue (`SceneComponent.K2_GetComponentToWorld` (`local.GrabCompRefLocal`)))
  (bind _output_get (set `local.GrabCompRefLocal` GtabComponentRef))
  (set `local.HandMeshRefLocal` HandMeshLocal)
  (if (`KismetSystemLibrary.IsValid` _output_get)
    ;[1 1 1] Snap to component
    ;;[1 1 1] Snap no inter
    (`SceneComponent.K2_SetWorldLocationAndRotation` (`local.HandMeshRefLocal`) (`KismetMathLibrary.TransformLocation` _returnvalue (.location HandDefaultRelTransf)) (`KismetMathLibrary.TransformRotation` _returnvalue (.rotation HandDefaultRelTransf)) false false)
    (return true)
    (else
      (return false))))

(fn `HCTraceIfTouchedSurfaceByIndex`
  (params (TraceDistance :type "Float (double-precision)" :default 1.2) (MoveStartTraceFrwd :type "Float (double-precision)" :default -1.8) (Index :type Integer))
  (returns (TraceBlocked :type Boolean) (DistanceBtwStartToImpact :type "Float (double-precision)"))
  (bind _s_handallbonenamesbase (`self.S_HandAllBoneNamesBase`))
  (bind _handmeshtocontrolref (`self.HandMeshToControlRef`))
  (bind _rotation (.rotation (`SceneComponent.GetSocketTransform` _handmeshtocontrolref (`.BoneName_47_1A2061D84E8FEED22A83A5AEED4639F1` (break `/Game/VRHandGrab/Blueprints/Structures/S_HandBoneRotation` (`|GetArrayItem` _s_handallbonenamesbase Index))) "RTS_World")))
  (bind _returnvalue (`KismetMathLibrary.GetRightVector` _rotation))
  (bind _returnvalue_2 (+ (+ (* _returnvalue (`self.Move Start TraceUp`)) (.location (`SceneComponent.GetSocketTransform` _handmeshtocontrolref (`.BoneName_47_1A2061D84E8FEED22A83A5AEED4639F1` (break `/Game/VRHandGrab/Blueprints/Structures/S_HandBoneRotation` (`|GetArrayItem` _s_handallbonenamesbase Index))) "RTS_World"))) (* (`KismetMathLibrary.GetForwardVector` _rotation) MoveStartTraceFrwd)))
  (if (`KismetArrayLibrary.Array_IsValidIndex` _s_handallbonenamesbase Index)
    (`/Engine/EditorBlueprintResources/StandardMacros.IsValid` _handmeshtocontrolref
      (:`Is Valid`
        (bind (_outhit _returnvalue_3) (`KismetSystemLibrary.BoxTraceSingle` :`Start` _returnvalue_2 :`End` (+ _returnvalue_2 (* _returnvalue TraceDistance)) :`HalfSize` (`KismetMathLibrary.MakeVector` (`self.FingerBoxTraceLength`) 0.0 (`self.FingerBoxTraceWidth`)) :`Orientation` _rotation :`TraceChannel` "TraceTypeQuery1" :`bIgnoreSelf` false :`DrawTime` 20.0)) ; X length y height z width
        (return _returnvalue_3 (`.Distance` (`GameplayStatics.BreakHitResult` _outhit))))
      (:`Is Not Valid`
        (`KismetSystemLibrary.PrintString` "AC_VRRealisticGrabHand: HCCheckIfTouchedSurface-> Hand mesh is not valid" true false (struct :`G` 0.66 :`B` 1.0 :`A` 1.0) 0.1)))))

(fn `HCUndoMoveFinger`
  (params (Index :type Integer) (FingerMovementSpeed :type "Float (double-precision)" :default 0.1))
  (returns (Success :type Boolean) (IndexModified :type Integer))
  (locals (AlphaSet :type "Float (double-precision)" :default 0.0))
  (bind _s_handallbonenamesbase (`self.S_HandAllBoneNamesBase`))
  (bind _output (`|GetArrayItem` _s_handallbonenamesbase Index))
  (if (`KismetArrayLibrary.Array_IsValidIndex` _s_handallbonenamesbase Index)
    (bind _output_get (set `local.AlphaSet` (`KismetMathLibrary.FClamp` (+ (`.Alpha_38_5439CFAD46D58980D75259BC215F4D5C` (break `/Game/VRHandGrab/Blueprints/Structures/S_HandBoneRotation` _output)) (* FingerMovementSpeed -1.0 (`GameplayStatics.GetWorldDeltaSeconds`) 100.0)))))
    (bind _structout (setmembers `/Game/VRHandGrab/Blueprints/Structures/S_HandBoneRotation` :`StructRef` _output :`Alpha` _output_get))
    (`KismetArrayLibrary.Array_Set` _s_handallbonenamesbase Index _structout)
    (return true Index)
    (else
      (return false 0))))

(fn `HCUpdate Hand Anim BP`
  (bind _handmeshtocontrolref (`self.HandMeshToControlRef`))
  (`/Engine/EditorBlueprintResources/StandardMacros.IsValid` _handmeshtocontrolref
    (:`Is Valid`
      (message `/Game/VRHandGrab/Blueprints/BPI_HandAnim.UpdateHandBones` (`SkeletalMeshComponent.GetAnimInstance` _handmeshtocontrolref) (`self.S_HandAllBoneNamesBase`)))
    (:`Is Not Valid`
      (`KismetSystemLibrary.PrintString` "AC_VRRealisticGrabHand: HCUpdate Hand Anim BP-> Hand mesh is not valid" true false (struct :`G` 0.66 :`B` 1.0 :`A` 1.0) 0.1))))

(fn `HCUpdateControllerPosAndGrabAnim`
  (params (GrabComponentRef :type "/Game/VRHandGrab/Blueprints/ACGrabComponent Object Reference") (MotionControllerRef :type "MotionControllerComponent Object Reference") (HandMeshToControlRef :type "SkeletalMeshComponent Object Reference"))
  (set `self.MotionControlRefTarget` MotionControllerRef)
  (set `self.HandMeshToControlRef` HandMeshToControlRef)
  (bind _output_get (set `self.Grab Component Ref` GrabComponentRef))
  (bind _customfingeralpha (`/Game/VRHandGrab/Blueprints/ACGrabComponent.CustomFingerAlpha` _output_get))
  ;[1 1 1] Custom alpha for fingers on begin play
  (if (> _customfingeralpha 0.0)
    (bind _output_get_2 (set `self.CurrCustomFingerAlphaInterp` (`KismetMathLibrary.FInterpTo` (`self.CurrCustomFingerAlphaInterp`) _customfingeralpha (`GameplayStatics.GetWorldDeltaSeconds`) 10.0)))
    (`self.SetCustomFingerAlpha` _output_get_2)
    (if (> _output_get_2 (/ _customfingeralpha 2.0))
      ;[1 1 1] If Grab type = snap and start grab simulate
      (bind _snapped (`self.HCSnapHandMeshToObj` (`local.GrabComponentRef`) (`self.HandMeshToControlRef`) (`self.Hand Rel Transform Default`) :!label _label))
      (bind _output_get_3 (set `self.HandSnappedToObject` _snapped))
      (if _output_get_3
        (`self.StartSimGrab` (`local.HandMeshToControlRef`))
        (else
          (`self.StopSimGrab`))))
    (else
      (goto _label))))

(fn `Init Comp`
  (params (HandMeshToControlRef :type "SkeletalMeshComponent Object Reference") (MotionControlRefTarget :type "MotionControllerComponent Object Reference") (Hand :type "EControllerHand Enum" :default "Left"))
  (set `self.Hand Rel Transform Default` (`SceneComponent.GetRelativeTransform` HandMeshToControlRef))
  (set `self.HandMeshToControlRef` HandMeshToControlRef)
  (set `self.MotionControlRefTarget` MotionControlRefTarget)
  (set `self.Hand` Hand)
  (return))

(fn `SetCustomFingerAlpha`
  (params (FingerAlpha :type "Float (double-precision)"))
  (for (_ _array_index) (`self.S_HandAllBoneNamesBase`)
    (`self.HCSetFingerAlpha` _array_index FingerAlpha))
  (`self.HCUpdate Hand Anim BP`)
  (return))

(fn `SimGrabOnTick`
  (params (AttachedActorRef :type "Actor Object Reference"))
  (locals (`Nearest ComponentTemp` :type "/Game/VRHandGrab/Blueprints/ACGrabComponent Object Reference") (AttachedActorLocal :type "Actor Object Reference"))
  (bind _nearest_component (`self.Nearest Component`))
  (bind _nearest_component_2 (`self.Nearest Component`))
  (set `local.AttachedActorLocal` AttachedActorRef)
  (`|ExecutionSequence`
    (:`then_0`
      (if (and (`KismetSystemLibrary.IsValid` (`local.AttachedActorLocal`)) (`KismetSystemLibrary.IsValid` (`self.Nearest Component`)))
        ;[0 1 0.5702] Hand simulation when item is in hand
        (`/Engine/EditorBlueprintResources/StandardMacros.IsValid` (`self.Nearest Component`) :!label _label
          (:`Is Valid`
            (if (and (== (`self.GetOwner` _nearest_component) (`local.AttachedActorLocal`)) (`/Game/VRHandGrab/Blueprints/ACGrabComponent.Enabled` _nearest_component))
              (switch `/Game/VRHandGrab/Blueprints/Enums/E_SnapTypeOnOverlap` (`/Game/VRHandGrab/Blueprints/ACGrabComponent.SnapTypeOnOverlap` (`self.Nearest Component`))
                (:`NewEnumerator2`
                  (`self.HCUpdateControllerPosAndGrabAnim` (`self.Nearest Component`) (`self.MotionControlRefTarget`) (`self.HandMeshToControlRef`) :!label _label_2))
                (:`NewEnumerator1`
                  (`self.StartSimGrab` (`self.HandMeshToControlRef`))
                  (set `self.HandSnappedToObject` false))
                (:`NewEnumerator3`
                  (goto _label_2))))))
        (else
          (bind _nearestcomponent (`/Game/VRHandGrab/Blueprints/BP_VRRealHandLibrary.MF_GetGrabCompNearMotionController` (`self.MotionControlRefTarget`) (`self.Hand`)))
          (set `self.Nearest Component` _nearestcomponent)
          (`local.AttachedActorLocal` ; Do if No items in hand, updated from grab component
            (:`then`
              (goto _label))
            (:`else`
              ;[0 1 0.5702] Hand  snap logic on overlap with item
              (`/Engine/EditorBlueprintResources/StandardMacros.IsValid` _nearest_component_2
                (:`Is Valid`
                  (if (`/Game/VRHandGrab/Blueprints/ACGrabComponent.Enabled` _nearest_component_2)
                    (`/Game/VRHandGrab/Blueprints/ACGrabComponent.OnOverlappedWithMCOnTick` _nearest_component_2 (`self.MotionControlRefTarget`))
                    (switch `/Game/VRHandGrab/Blueprints/Enums/E_SnapTypeOnOverlap` (`/Game/VRHandGrab/Blueprints/ACGrabComponent.SnapTypeOnOverlap` (`self.Nearest Component`))
                      (:`NewEnumerator2`
                        (`self.HCUpdateControllerPosAndGrabAnim` (`self.Nearest Component`) (`self.MotionControlRefTarget`) (`self.HandMeshToControlRef`)))
                      (:`NewEnumerator1`
                        (`self.StartSimGrab` (`self.HandMeshToControlRef`))
                        (set `self.HandSnappedToObject` false))
                      (:`NewEnumerator3`
                        (`self.StopSimGrab`)
                        (set `self.HandSnappedToObject` false)))
                    (else
                      (`self.StopSimGrab` :!label _label_3))))
                (:`Is Not Valid`
                  (goto _label_3))))))))
    (:`then_1`
      (`self.TryResetHandRelTransform`))))