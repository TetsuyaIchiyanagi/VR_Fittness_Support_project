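; BP_Fitness_Camera is the player's view camera in the VR fitness game, taking over as view target on BeginPlay.
; Each tick, CameraMirrorMode selects between a mirror view and a spring-arm follow view.
; Mirror mode collapses the arm, hides BP_Mirro and reflects the head socket's XY through the mirror's location at head height with fixed yaw.
; Otherwise it follows above the pawn using control rotation and shows the mirror.
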(event `self.ReceiveBeginPlay`
  (`PlayerController.SetViewTargetWithBlend` (`GameplayStatics.GetPlayerController` 0) self 0.0 "VTBlend_Linear" 0.0 false)
  (set `self.SkeletalMesh` (`Character.Mesh` (`GameplayStatics.GetPlayerCharacter` 0)))
  (bind _returnvalue (`GameplayStatics.GetActorOfClass` "/Game/VR_Fitness/00_Blueprints/BP_Mirro.BP_Mirro_C"))
  (set `self.BP_mirror` _returnvalue))

(event `self.ReceiveTick`
  (params (DeltaSeconds :type "Float (single-precision)"))
  (bind _returnvalue (`GameplayStatics.GetPlayerPawn` 0))
  (bind (_returnvalue_x _returnvalue_y _returnvalue_z) (`KismetMathLibrary.BreakVector` (`self.K2_GetActorLocation` _returnvalue)))
  (bind _returnvalue_2 (`self.K2_GetActorLocation` (`self.BP_mirror`)))
  (bind (_returnvalue_x_2 _returnvalue_y_2) (`KismetMathLibrary.BreakVector` (+ _returnvalue_2 (- _returnvalue_2 (.location (`SceneComponent.GetSocketTransform` (`self.SkeletalMesh`) "head" "RTS_World"))))))
  (if (`self.CameraMirrorMode`)
    (set `SpringArmComponent.TargetArmLength` 0.0 (`self.SpringArm`))
    (`self.K2_SetActorLocationAndRotation` (`KismetMathLibrary.MakeVector` _returnvalue_x_2 _returnvalue_y_2 (.z (.location (`SceneComponent.GetSocketTransform` (`self.SkeletalMesh`) "head" "RTS_World")))) (`KismetMathLibrary.MakeRotator` 0.0 0.0 -90.0) true)
    (`self.SetActorHiddenInGame` (`self.BP_mirror`) true)
    (else
      (set `SpringArmComponent.TargetArmLength` 100.0 (`self.SpringArm`))
      (`self.K2_SetActorLocationAndRotation` (`KismetMathLibrary.MakeVector` (+ _returnvalue_x 0.0) _returnvalue_y (+ _returnvalue_z 50.0)) (`Pawn.GetControlRotation` _returnvalue) true)
      (`self.SetActorHiddenInGame` (`self.BP_mirror`) false))))

(fn `UserConstructionScript`)