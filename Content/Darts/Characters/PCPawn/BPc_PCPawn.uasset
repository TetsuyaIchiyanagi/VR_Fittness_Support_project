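; BPc_PCPawn is a pawn in the Darts game, apparently for PC play, that moves from player axis input.
; The MoveForward and MoveRight axes offset its location along its forward and right vectors, scaled by a fixed step.
; Movement sets the actor location directly every frame, without sweep collision or delta-time scaling.
; Tick and overlap events are disabled placeholders, and the construction script only calls its parent.
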(event `InputAxis|MoveForward`
  (params (AxisValue :type "Float (single-precision)"))
  (`self.K2_SetActorLocation` (+ (* (`self.GetActorForwardVector`) (* 10 AxisValue)) (`self.K2_GetActorLocation`))))

(event `InputAxis|MoveRight`
  (params (AxisValue :type "Float (single-precision)"))
  (`self.K2_SetActorLocation` (+ (* (`self.GetActorRightVector`) (* 10 AxisValue)) (`self.K2_GetActorLocation`))))

(fn `UserConstructionScript`
  (`parent.UserConstructionScript`))