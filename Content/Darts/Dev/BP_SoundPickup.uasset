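; Sound-emitting pickup actor that plays audio with animated wave meshes when picked up.
; Pickup disables cylinder physics, attaches the root to the given component and starts audio and a timeline; Drop restores physics, detaches and optionally stops both.
; The timeline alpha feeds InterpSoundWaves, which moves and scales four meshes from transforms cached at BeginPlay.
; Per-index range remapping staggers their rates from one alpha, suggesting waves spreading outward.
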(event `self.ReceiveBeginPlay`
  ;[1 1 1] Get a reference to the sound wave transforms
  (bind _output_get (set `self.Sound Waves Prepresentations` (`|MakeArray` (`self.SM_Ceiling0`) (`self.SM_Ceiling1`) (`self.SM_Ceiling2`) (`self.SM_Ceiling3`))))
  (for _array_element _output_get
    (`KismetArrayLibrary.Array_Add` (`self.SoundWaveStart`) (`SceneComponent.GetRelativeTransform` _array_element))))

(event `/Game/VirtualRealityBP/Blueprints/PickupActorInterface.Pickup`
  (params (AttachTo :type "SceneComponent Object Reference"))
  (`PrimitiveComponent.SetSimulatePhysics` (`self.CylinderToHold`) false)
  (`SceneComponent.K2_AttachToComponent` (`self.RootComponent`) AttachTo "None" "KeepWorld" "KeepWorld" "KeepWorld" false)
  (`|ExecutionSequence`
    (:`then_0`
      (bind (_direction _alpha) (`Timeline|RepresentSound_TL`)
        (:`Update`
          (`self.InterpSoundWaves` _alpha))))
    (:`then_1`
      (`AudioComponent.Play` (`self.Audio`) 0.0))))

(event `/Game/VirtualRealityBP/Blueprints/PickupActorInterface.Drop`
  (`PrimitiveComponent.SetSimulatePhysics` (`self.CylinderToHold`) true)
  (`self.K2_DetachFromActor` "KeepWorld" "KeepWorld" "KeepWorld")
  (if (`self.StopPlayingWhenDropped`)
    (`TimelineComponent.Stop` (`self.RepresentSound_TL`))
    (`AudioComponent.Stop` (`self.Audio`))))

(fn `InterpSoundWaves`
  (params (Alpha :type "Float (double-precision)"))
  ;[1 0.8518 0] Shift the sound representations at differant rates from an alpha variable in a Timeline
  (for (_array_element _array_index) (`self.Sound Waves Prepresentations`)
    (bind (_output_location _output_rotation _output_scale) (`KismetMathLibrary.BreakTransform` (`|GetArrayItem` (`self.SoundWaveStart`) _array_index)))
    (bind _returnvalue (`KismetMathLibrary.MapRangeClamped` Alpha -0.5 (select `int` _array_index :`0` 0.1 :`1` 0.2 :`2` 0.5 :`3` 1.0 :!type "Float (single-precision)") -0.5 1.0))
    (`SceneComponent.K2_SetRelativeTransform` _array_element (`KismetMathLibrary.MakeTransform` (`KismetMathLibrary.VLerp` _output_location (`KismetMathLibrary.MakeVector` (.x _output_location) (* (.y _output_location) 2.0) (.z _output_location)) _returnvalue) (struct :`Roll` 90.0) (`KismetMathLibrary.VLerp` _output_scale (* _output_scale 2.0) _returnvalue)) false false)))

(fn `UserConstructionScript`)