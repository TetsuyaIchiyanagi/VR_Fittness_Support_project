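; Dartboard actor that reports dart hits to GameMode_Darts, flagging whether each landed in the current bonus quadrant.
; DeterminQuadrandHit maps the hit's atan2 angle around the Arrow in the X-Z plane to a quadrant through nested comparisons, all against the same threshold.
; A bonus hit triggers SetNewBonus, which removes the current quadrant from a shuffled candidate list and picks a replacement.
; BeginPlay creates a dynamic board material, otherwise unused here.
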(event `self.ReceiveBeginPlay`
  (bind _returnvalue (`PrimitiveComponent.CreateDynamicMaterialInstance` (`self.Dartboard`) 0 null "None"))
  (set `self.Dartboard_Material` _returnvalue))

(event `DartBoardHit`
  (params (ComponentHit :type "PrimitiveComponent Object Reference") (HitLocation :type "Vector Structure"))
  (if (== null (`self.Dartboard`))
    (bind _quadrant (`self.DeterminQuadrandHit` HitLocation))
    (bind _asgame_mode_darts (cast `/Game/Darts/Core/GameMode_Darts` (`GameplayStatics.GetGameMode`)))
    (bind _returnvalue (== _quadrant (`self.BounusQuadrant`)))
    (`/Game/Darts/Core/GameMode_Darts.PlayerHasScored2` _asgame_mode_darts _returnvalue)
    (if _returnvalue
      (`self.SetNewBonus`))
    (else
      (`KismetSystemLibrary.PrintString` "FALSEEEEEEEEEEEE"))))

(event `SetNewBonus`
  (bind _possiblequadrants (`self.PossibleQuadrants`))
  ;[1 1 1] Randomly select the new quadrant for bonus points. Make sure that the current bonus is removed to avoid replication
  (bind _output_get (set `self.PossibleQuadrants` (`|MakeArray` 0 0 0 0 0)))
  (`KismetArrayLibrary.Array_RemoveItem` _output_get (`self.BounusQuadrant`))
  (`KismetArrayLibrary.Array_Shuffle` _possiblequadrants)
  (bind _output_get_2 (set `self.BounusQuadrant` (`|GetArrayItem` _possiblequadrants (`KismetMathLibrary.RandomIntegerInRange` 0 2))))
  (`KismetSystemLibrary.PrintString` (`KismetStringLibrary.Conv_IntToString` _output_get_2)))

(fn `DeterminQuadrandHit`
  (params (HitLocation :type "Vector Structure"))
  (returns (Quadrant :type Integer))
  (bind (_returnvalue_x _returnvalue_y _returnvalue_z) (`KismetMathLibrary.BreakVector` (`SceneComponent.K2_GetComponentLocation` (`self.Arrow`))))
  (bind (_returnvalue_x_2 _returnvalue_y_2) (`KismetMathLibrary.BreakVector2D` (- (`KismetMathLibrary.MakeVector2D` _returnvalue_x _returnvalue_z) (`KismetMathLibrary.MakeVector2D` HitLocation_X HitLocation_Z))))
  (set `self.Result_local` (+ (`KismetMathLibrary.DegAtan2` _returnvalue_x_2 _returnvalue_y_2) 180.0))
  (`/Engine/EditorBlueprintResources/StandardMacros.CompareFloat` (`self.Result_local`) 90.0
    (:`>`
      _)
    (:`==`
      _)
    (:`<`
      (return 2)))
  (`/Engine/EditorBlueprintResources/StandardMacros.CompareFloat` (`self.Result_local`) 90.0
    (:`>`
      _)
    (:`==`
      _)
    (:`<`
      (return 3)))
  (`/Engine/EditorBlueprintResources/StandardMacros.CompareFloat` (`self.Result_local`) 90.0
    (:`>`
      (return 1))
    (:`<`
      (return 4))))

(fn `UserConstructionScript`)