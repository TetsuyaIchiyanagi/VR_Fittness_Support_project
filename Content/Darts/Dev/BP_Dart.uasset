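; BP_Dart is a throwable dart that can be picked up, attached to the hand and released with physics.
; On release it fires DartThrown and starts a 60 Hz timer to align the dart with its velocity and line-trace ahead of the tip.
; A dartboard hit is reported to BP_Dartboard with impact point and component.
; That hit, or a static mesh collision, freezes the dart and sets a short lifespan.
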(event `/Game/Darts/Characters/VRPawn/PickupActorInterface_Darts.Pickup`
  (params (AttachTo :type "SceneComponent Object Reference") (skeletalMesh :type "SkeletalMesh Object Reference"))
  ;[1 1 1] User picked up the dart
  (`PrimitiveComponent.SetSimulatePhysics` (`self.Dart_Controller`) false)
  (`self.K2_AttachToComponent` AttachTo "hand_r" "SnapToTarget" "SnapToTarget" "KeepWorld"))

(event `/Game/Darts/Characters/VRPawn/PickupActorInterface_Darts.Drop`
  ;[1 1 1] User dropped or threw the dart
  (`PrimitiveComponent.SetSimulatePhysics` (`self.Dart_Controller`) true)
  (`self.K2_DetachFromActor` "KeepWorld" "KeepWorld" "KeepWorld")
  (bind _returnvalue (`KismetSystemLibrary.K2_SetTimerDelegate` (`|CreateDelegate` :!event `Adjust Rotation From Throw`) (/ 1.0 60.0) true))
  (set `self.DartRotationTimer` _returnvalue)
  (`self.DartThrown`))

(event `Adjust Rotation From Throw`
  (`SceneComponent.K2_SetWorldRotation` (`self.Dart_Controller`) (`KismetMathLibrary.MakeRotFromXZ` (`SceneComponent.GetComponentVelocity` (`self.Dart_Controller`)) (0.0 0.0 0.0)) false false)
  (`SceneComponent.K2_SetRelativeRotation` (`self.Dart_Rotator`) (struct :`Pitch` 90.0 :`Yaw` -180.0 :`Roll` -180.0) false false)
  (`self.CheckIfHitSomething`))

(event `CheckIfHitSomething`
  (bind _arrow (`self.Arrow`))
  (bind _returnvalue (`SceneComponent.K2_GetComponentLocation` _arrow))
  (bind _outhit (`KismetSystemLibrary.LineTraceSingle` _returnvalue (+ _returnvalue (* (`SceneComponent.GetForwardVector` _arrow) 15.0)) "TraceTypeQuery1"))
  (bind (_bblockinghit _binitialoverlap _time _distance _location _impactpoint _normal _impactnormal _physmat _hitactor _hitcomponent) (`GameplayStatics.BreakHitResult` _outhit))
  (if _bblockinghit
    ;[1 1 1] True if what was hit was the dartboard
    (bind _asbp_dartboard (cast `/Game/Darts/Dev/BP_Dartboard` _hitactor))
    (`/Game/Darts/Dev/BP_Dartboard.Dartboard Hit` _asbp_dartboard _impactpoint _hitcomponent)
    (`self.StopDartMotion`)))

(event `StopDartMotion`
  (`PrimitiveComponent.SetSimulatePhysics` (`self.Dart_Controller`) false)
  (`KismetSystemLibrary.K2_PauseTimerHandle` (`self.DartRotationTimer`))
  (`self.SetLifeSpan` 5.0))

(event `self.Sphere2.OnComponentHit`
  (params (HitComponent :type "PrimitiveComponent Object Reference") (OtherActor :type "Actor Object Reference") (OtherComp :type "PrimitiveComponent Object Reference") (NormalImpulse :type "Vector Structure") (Hit :type "HitResult Structure (by ref)"))
  ;[1 1 1] If dart hits something that is not the dartboard, stop motion
  (cast `StaticMeshActor` OtherActor)
  (`self.StopDartMotion`))

(fn `UserConstructionScript`)