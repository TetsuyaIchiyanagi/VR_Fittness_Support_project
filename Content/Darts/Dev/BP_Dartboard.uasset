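; Dartboard actor for a darts minigame that handles hits, a moving bonus quadrant, score totals and game time.
; Hits resolve to a quadrant via atan2 around an Arrow component and go to GameMode_Darts, with bonus hits picking a different quadrant.
; Horizontal and vertical widgets display results, while the board rotates and toggles a dynamic material parameter to reveal the bonus.
; A looping timer starts on first hit; game over triggers the leaderboard update.
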(event `self.ReceiveBeginPlay`
  ;[1 1 1] Reference to the material of the dartboard
  (bind _returnvalue (`PrimitiveComponent.CreateDynamicMaterialInstance` (`self.Dartboard`) 0 null "None"))
  (set `self.Dartboard Material` _returnvalue)
  ;[1 1 1] Reference the two widgets in our two boards
  (bind _output_get (set `self.W_Darts_Horiz` (cast `/Game/Darts/UI/UMG/DartGame/W_Darts_Main_Horiz` (`WidgetComponent.GetUserWidgetObject` (`self.Widget`)) :!pure true)))
  (set `/Game/Darts/UI/UMG/DartGame/W_Darts_Main_Horiz.BP_Dartboard` self _output_get)
  (set `self.W_Darts_Vert` (cast `/Game/Darts/UI/UMG/DartGame/W_Darts_Main_Vert` (`WidgetComponent.GetUserWidgetObject` (`/Game/Darts/UI/Actors/BP_GameBoardData.Widget` (`self.GameBoardData`))) :!pure true))
  (`self.SetNewBonus`))

(event `Dartboard Hit`
  (params (`Hit Location` :type "Vector Structure") (`Component Hit` :type "PrimitiveComponent Object Reference"))
  (bind _returnvalue (== `Component Hit` (`self.Dartboard`)))
  ;[1 1 1] Dartboard was hit!
  (`/Game/Darts/UI/UMG/DartGame/W_Darts_Main_Vert.UpdateThrows` (`self.W_Darts_Vert`) _returnvalue)
  (if _returnvalue
    ;[1 1 1] Check if the player hit the bonus quadrant and pass the data onto other Blueprints for update
    (bind _quadrant (`self.DetermineQuadrant of Hit` `Hit Location`))
    (bind _asgame_mode_darts (cast `/Game/Darts/Core/GameMode_Darts` (`GameplayStatics.GetGameMode`)))
    (bind _returnvalue_2 (== _quadrant (`self.BonusQuadrant`)))
    (`/Game/Darts/Core/GameMode_Darts.PlayerHasScored` _asgame_mode_darts _returnvalue_2 self)
    (`self.PlayHitAnimation` _returnvalue_2)
    (if _returnvalue_2
      (`self.SetNewBonus`))
    (`self.StartGameTimer`)))

(event `SetNewBonus`
  (bind _possiblequadrants (`self.PossibleQuadrants`))
  ;[1 1 1] Randomly select the new quadrant for bonus points. Make sure that the current bonus is removed to avoid replication
  (bind _output_get (set `self.PossibleQuadrants` (`|MakeArray` 1 2 3 4)))
  (`KismetArrayLibrary.Array_RemoveItem` _output_get (`self.BonusQuadrant`))
  (`KismetArrayLibrary.Array_Shuffle` _possiblequadrants)
  (bind _output_get_2 (set `self.BonusQuadrant` (`|GetArrayItem` _possiblequadrants (`KismetMathLibrary.RandomIntegerInRange` 0 2))))
  (`/Game/Darts/UI/UMG/DartGame/W_Darts_Main_Horiz.SetNewBonus` (`self.W_Darts_Horiz`) _output_get_2)
  (`self.ToggleShowingBonus` false))

(event `SpinBoard`
  (params (`Y Rotation` :type "Float (double-precision)"))
  (bind _dartboard (`self.Dartboard`))
  ;[1 1 1] When the bonus quadrant is displayed, rotate the board so the red texture is in the correct spot.
  (`/Engine/EditorBlueprintResources/StandardMacros.IsValid` _dartboard
    (:`Is Valid`
      (`SceneComponent.K2_SetRelativeRotation` _dartboard (`KismetMathLibrary.MakeRotator` -90.0 (+ `Y Rotation` 90.0)) false false)
      (`self.ToggleShowingBonus` true))))

(event `ToggleShowingBonus`
  (params (ShowBonus :type Boolean))
  ;[1 1 1] When the new quadrant is spinning, hide the red on the board. When it has found the new spot, display the red
  (`KismetSystemLibrary.Delay` (`KismetMathLibrary.SelectFloat` 0.0 1.0 ShowBonus))
  (`MaterialInstanceDynamic.SetScalarParameterValue` (`self.Dartboard Material`) "ShowBonus" (`KismetMathLibrary.SelectFloat` 1.0 0.0 ShowBonus)))

(event `UpdateScore`
  (params (PointsAdded :type Integer) (BonusHit :type Boolean))
  ;[1 1 1] Update the offical score count, seperate it by score type, and send data to Widget
  (bind _output_get (set `self.PlayerScore` (+ (`self.PlayerScore`) PointsAdded)))
  (`/Game/Darts/UI/UMG/DartGame/W_Darts_Main_Horiz.UpdateScore` (`self.W_Darts_Horiz`) _output_get BonusHit)
  (if BonusHit
    (set `self.BonusTotal` (+ (`self.BonusTotal`) PointsAdded))
    (else
      (set `self.StandardTotal` (+ PointsAdded (`self.StandardTotal`)))))
  (`/Game/Darts/UI/UMG/DartGame/W_Darts_Main_Vert.UpdateUserScore` (`self.W_Darts_Vert`) (`self.BonusTotal`) (`self.StandardTotal`)))

(event `StartGameTimer`
  ;[1 1 1] Set timer to inrease game time
  (if (not (`KismetSystemLibrary.K2_IsValidTimerHandle` (`self.GameTimer`)))
    (bind _returnvalue (`KismetSystemLibrary.K2_SetTimerDelegate` (delegate `IncrementGameTime`) 1.0 true))
    (set `self.GameTimer` _returnvalue)))

(event `IncrementGameTime`
  ;[1 1 1] Increment Game Time in seconds and send result to the Widget
  (if (`self.GameOver`)
    (`KismetSystemLibrary.K2_PauseTimerHandle` (`self.GameTimer`))
    ;[1 1 1] Update Leaderboard with game time
    (`/Game/Darts/Core/GameMode_Darts.UpdateLeaderboard` :`self` (cast `/Game/Darts/Core/GameMode_Darts` (`GameplayStatics.GetGameMode`) :!pure true))
    (else
      (set `self.NewTimer` (+ (`self.NewTimer`) (`KismetMathLibrary.MakeTimespan` 0 0 0 1)))
      (`/Game/Darts/UI/UMG/DartGame/W_Darts_Main_Horiz.UpdateTime` (`self.W_Darts_Horiz`) (`self.NewTimer`)))))

(event `PlayHitAnimation`
  (params (Bonus :type Boolean))
  (bind _w_darts_horiz (`self.W_Darts_Horiz`))
  ;[1 1 1] When Player Score, play animation depending on if the bonus was hit or not
  (`UserWidget.PlayAnimation` _w_darts_horiz (select `bool` Bonus :`false` (`/Game/Darts/UI/UMG/DartGame/W_Darts_Main_Horiz.HIT` _w_darts_horiz) :`true` (`/Game/Darts/UI/UMG/DartGame/W_Darts_Main_Horiz.BonusHit` _w_darts_horiz)) 0.0 1 "Forward" 1.0 false))

(event `GameHasEnded`
  (bind _w_darts_horiz (`self.W_Darts_Horiz`))
  ;[1 1 1] Play Game Over Animation
  (set `self.GameOver` true)
  (`UserWidget.PlayAnimation` _w_darts_horiz (`/Game/Darts/UI/UMG/DartGame/W_Darts_Main_Horiz.GameOver` _w_darts_horiz) 0.0 1 "Forward" 1.0 false)
  (`ActorComponent.K2_DestroyComponent` (`self.Dartboard`)))

(fn `DetermineQuadrant of Hit`
  (params (`Hit Location` :type "Vector Structure"))
  (returns (Quadrant :type Integer))
  (locals (Result :type "Float (double-precision)" :default 0.0))
  (bind (_returnvalue_x _returnvalue_y _returnvalue_z) (`KismetMathLibrary.BreakVector` (`SceneComponent.K2_GetComponentLocation` (`self.Arrow`))))
  (bind (_returnvalue_x_2 _returnvalue_y_2) (`KismetMathLibrary.BreakVector2D` (- (`KismetMathLibrary.MakeVector2D` _returnvalue_x _returnvalue_z) (`KismetMathLibrary.MakeVector2D` `Hit Location_X` `Hit Location_Z`))))
  ;[1 0.8518 0] Going to create a counterclockwise float value from -180 - 180
  ;
  ; ATAN2(y,x) returns the arc tangent of the two numbers x and y. It is similar to calculating the arc tangent of y / x, except that the signs of both arguments are used to determine the quadrant of the result. The result is an angle expressed in degrees
  (set `local.Result` (+ (`KismetMathLibrary.DegAtan2` _returnvalue_x_2 _returnvalue_y_2) 180.0))
  (`/Engine/EditorBlueprintResources/StandardMacros.CompareFloat` (`local.Result`) 90.0
    (:`>`
      _)
    (:`==`
      _)
    (:`<`
      (return 2)))
  (`/Engine/EditorBlueprintResources/StandardMacros.CompareFloat` (`local.Result`) 180.0
    (:`>`
      _)
    (:`==`
      _)
    (:`<`
      (return 3)))
  (`/Engine/EditorBlueprintResources/StandardMacros.CompareFloat` (`local.Result`) 270.0
    (:`>`
      _)
    (:`==`
      _)
    (:`<`
      (return 4)))
  (return 1))

(fn `UserConstructionScript`)