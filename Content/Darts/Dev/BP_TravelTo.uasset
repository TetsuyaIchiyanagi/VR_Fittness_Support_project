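; Level-travel trigger for the Darts game that moves the player to a soft-referenced level on box overlap, deep-link entry or game over.
; Travel async-loads the level behind a VR splash screen, briefly holds it, then opens the level by name from the reference's path.
; Deep-link entry targets the game stage as a listen server, while game over waits a GameInstance-configured delay.
; The construction script sizes the box and keeps it on the ground.
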(event `self.ReceiveBeginPlay`
  (`parent.ReceiveBeginPlay`)
  ;[1 1 1] If there is a loading Screen
  (`KismetSystemLibrary.Delay` 1.0)
  (`XRLoadingScreenFunctionLibrary.HideLoadingScreen`))

(event `self.TravelTo`
  (bind (_pathpart _filenamepart _extensionpart) (`BlueprintPathsLibrary.Split` (`KismetSystemLibrary.Conv_SoftObjectReferenceToString` (`self.Course Level To Travel To`))))
  ;[0.03991 0.3802 0] Only for testing level changing logic
  ;[1 1 1] Load the level in the background for speed
  (`|LoadAsset` (`self.Course Level To Travel To`) :!label _label
    (:`then`
      ;[1 1 1] Create and how loading screen to player
      (`OculusFunctionLibrary.AddLoadingSplashScreen` "/Game/Darts/UI/Textures/Unreal_Logomark.Unreal_Logomark" (1.0 0.0 1.5) (struct) (0.3 0.3) (struct) true)
      (`XRLoadingScreenFunctionLibrary.ShowLoadingScreen`))
    (:`Completed`
      ;[1 1 1] Artificially delay level change so the player sees the splash screen
      (`KismetSystemLibrary.Delay` 1.0)
      ;[1 1 1] Identify the path of the SoftObject reference and provide to the Open Level node
      (`GameplayStatics.OpenLevel` (`KismetStringLibrary.Conv_StringToName` (`KismetStringLibrary.Concat_StrStr` _pathpart "/" _extensionpart)) true (`self.TravelOption`)))))

(event `self.Box.OnComponentBeginOverlap`
  (params (OverlappedComponent :type "PrimitiveComponent Object Reference") (OtherActor :type "Actor Object Reference") (OtherComp :type "PrimitiveComponent Object Reference") (OtherBodyIndex :type Integer) (bFromSweep :type Boolean) (SweepResult :type "HitResult Structure (by ref)"))
  ;[0.03991 0.3802 0] Basic level change. No rules for  success
  (if (`KismetSystemLibrary.IsValidSoftObjectReference` (`self.Course Level To Travel To`))
    ;[1 1 1] Only collide with the Player
    (cast `/Game/Darts/Characters/ParentPawn/BPP_Pawn_Darts` OtherActor)
    (goto _label)))

(event `self.PlayerEnteredViaDeepLink`
  ;[1 1 1] PlayerArrivedVieDeeplink
  (set `self.Course Level To Travel To` "/Game/Darts/Maps/CourseZero/C0_GameStage.C0_GameStage")
  ;;[1 1 1] Start the level as a listen server
  (set `self.TravelOption` "listen")
  (`self.TravelTo`))

(event `self.GameOver`
  ;[1 1 1] Called from Gamemode when the game has ended
  (`KismetSystemLibrary.Delay` 1.0)
  (if (`KismetSystemLibrary.IsValidSoftObjectReference` (`self.Course Level To Travel To`))
    (bind _asgame_instance_darts (cast `/Game/Darts/Core/GameInstance_Darts` (`GameplayStatics.GetGameInstance`)))
    ;;[1 1 1] Delay before travel
    (`KismetSystemLibrary.Delay` (`.AfterGameover_Delaybeforetravelinseconds_55_2087DB3B4F7EC357CCAEA585AA9E4938` (break `/Game/Darts/Dev/Structure/Struc_VRPlayerSettings` (`/Game/Darts/Core/GameInstance_Darts.Struc_VRPlayerSettings` _asgame_instance_darts))))
    (`self.TravelTo`)))

(fn `UserConstructionScript`
  (bind _box (`self.Box`))
  (bind _boxextent (`self.BoxExtent`))
  (`parent.UserConstructionScript`)
  ;[1 1 1] Set the size of the collision
  (`BoxComponent.SetBoxExtent` _box _boxextent true)
  ;[1 1 1] Taking the Z extent of the box and using it to move the box up so it is always on the "ground"
  (`SceneComponent.K2_SetRelativeLocation` _box (`KismetMathLibrary.MakeVector` 0.0 0.0 (.z _boxextent)) false false))