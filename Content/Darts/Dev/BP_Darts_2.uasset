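; Throwable dart actor that can be picked up by attaching to a given component, then dropped with physics on.
; Dropping starts a looping 60 Hz timer; the rotation-adjust event resets orientation and runs a zero-length line trace at the arrow, reporting dartboard hits to BP_DartsBoard_2.
; Sphere hits on static mesh actors stop physics, pause the timer, set a short lifespan and fire DartThrown.
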(event `/Game/Darts/Characters/VRPawn/PickupActorInterface_Darts.Pickup`
  (params (AttachTo :type "SceneComponent Object Reference") (skeletalMesh :type "SkeletalMesh Object Reference"))
  (`PrimitiveComponent.SetSimulatePhysics` (`self.Darts_controler`) false)
  (`SceneComponent.K2_AttachToComponent` (`self.K2_GetRootComponent`) AttachTo "None" "KeepWorld" "KeepWorld" "KeepWorld" false))

(event `/Game/Darts/Characters/VRPawn/PickupActorInterface_Darts.Drop`
  (`PrimitiveComponent.SetSimulatePhysics` (`self.Darts_controler`) true)
  (`self.K2_DetachFromActor` "KeepWorld" "KeepWorld" "KeepWorld")
  (bind _returnvalue (`KismetSystemLibrary.K2_SetTimerDelegate` (`|CreateDelegate` :!event `Adjust Rotation From Throw`) (/ 1.0 60.0) true))
  (set `self.DartRotationTimer` _returnvalue))

(event `Adjust Rotation From Throw`
  (`SceneComponent.K2_SetWorldRotation` :`self` (`self.Darts_controler`))
  (`SceneComponent.K2_SetRelativeRotation` (`self.Darts_rotator`) (struct :`Pitch` 90.0 :`Yaw` -180.0 :`Roll` -180.0) false false)
  (`self.CheckIfHitSomething`))

(event `CheckIfHitSomething`
  (bind _returnvalue (`SceneComponent.K2_GetComponentLocation` (`self.Arrow`)))
  (bind _outhit (`KismetSystemLibrary.LineTraceSingle` _returnvalue (+ _returnvalue 0) "TraceTypeQuery1"))
  (bind (_bblockinghit _binitialoverlap _time _distance _location _impactpoint _normal _impactnormal _physmat _hitactor) (`GameplayStatics.BreakHitResult` _outhit))
  (if _bblockinghit
    (bind _asbp_darts_board_2 (cast `/Game/Darts/Dev/BP_DartsBoard_2` _hitactor))
    (`/Game/Darts/Dev/BP_DartsBoard_2.DartBoardHit` _asbp_darts_board_2 null _impactpoint)))

(event `StopDartMotion`
  (`PrimitiveComponent.SetSimulatePhysics` (`self.Darts_controler`) false)
  (`KismetSystemLibrary.K2_PauseTimerHandle` (`self.DartRotationTimer`))
  (`self.SetLifeSpan` 5.0)
  (`self.DartThrown`))

(event `self.Sphere.OnComponentHit`
  (params (HitComponent :type "PrimitiveComponent Object Reference") (OtherActor :type "Actor Object Reference") (OtherComp :type "PrimitiveComponent Object Reference") (NormalImpulse :type "Vector Structure") (Hit :type "HitResult Structure (by ref)"))
  (cast `StaticMeshActor` OtherActor)
  (`self.StopDartMotion`))

(fn `BP_Darts_2_AutoGenFunc`)

(fn `UserConstructionScript`)